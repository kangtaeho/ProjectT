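; Enemy character Blueprint that patrols around its spawn point, chases a target and attacks it in melee or ranged montages within AttackRange.
; Patrol loops random reachable-point moves with random pauses until OnAggroPulled, which AI Perception triggers for CB_Character when Aggressive.
; PerformAttack faces the target, plays a random montage, then repeats or closes in.
; A looping timer leash-checks distance from spawn, calling OnReset to run home and resume patrol.
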(event `self.ReceiveBeginPlay`
  ;[1 1 1] 초기화
  (set `self.StartingLocation` (`self.K2_GetActorLocation`))
  (set `CharacterMovementComponent.MaxWalkSpeed` (`self.PatrolWalkSpeed`) (`self.CharacterMovement`))
  (`self.Patrol`))

(event `Patrol`
  ;[1 1 1] 패트롤 모드
  (`|AIMoveTo` self (`NavigationSystem.K2_GetRandomReachablePointInRadius` (`self.StartingLocation`) (`self.PatrolRadius`))
    (:`then`
      (if (`self.IsPatroling`)
        (`KismetSystemLibrary.Delay` (`KismetMathLibrary.RandomFloatInRange` 2.0 4.0))
        (`self.Patrol`)))))

(event `OnAggroPulled`
  (params (Target :type "Actor Object Reference"))
  ;[1 1 1] 어그로 끌었냐?
  (if (and (not (`self.WasAggroed?`)) (not (`self.IsRunningBack?`)))
    (set `self.IsPatroling` false)
    (set `self.WasAggroed?` true)
    (set `self.TargetActor` Target)
    (set `CharacterMovementComponent.MaxWalkSpeed` (`self.AggroedWalkSpeed`) (`self.CharacterMovement`))
    (bind _returnvalue (`KismetSystemLibrary.K2_SetTimer` self "FollowTargetDistance" 1.0 true))
    (set `self.FollowDistanceTimer` _returnvalue)
    (if (`self.InAttackRange?`)
      (`self.PerformAttack`)
      (else
        (`|AIMoveTo` self (0.0 0.0 0.0) (`self.TargetActor`) (`self.AttackRange`)
          (:`OnSuccess`
            (`self.PerformAttack`)))))))

(event `PerformAttack`
  ;[1 1 1] 애니메이션 바뀌면서 공격
  (if (not (`self.IsDead?`))
    (`self.K2_SetActorRotation` (`KismetMathLibrary.FindLookAtRotation` (`self.K2_GetActorLocation` self) (`self.K2_GetActorLocation` (`self.TargetActor`))))
    (bind _output_get (set `self.CurrentAttackMontage` (`|GetArrayItem` (`self.AttackAnimation`) (`self.GetNextAnimation`))))
    (`self.PlayAnimMontage` _output_get)
    (`KismetSystemLibrary.Delay` (`AnimSequenceBase.SequenceLength` _output_get))
    (if (`self.InAttackRange?`)
      (`self.PerformAttack`)
      (else
        (`|AIMoveTo` self (0.0 0.0 0.0) (`self.TargetActor`) (`self.AttackRange`)
          (:`OnSuccess`
            (`self.PerformAttack`)))))))

(event `OnReset`
  ;[1 1 1] 어그로 중지(다시 패트롤)
  (set `self.IsRunningBack?` true)
  (`KismetSystemLibrary.K2_ClearAndInvalidateTimerHandle` (`self.FollowDistanceTimer`))
  (set `self.TargetActor` null)
  (set `self.WasAggroed?` false)
  (`|AIMoveTo` self (`self.StartingLocation`)
    (:`then`
      (set `CharacterMovementComponent.MaxWalkSpeed` (`self.PatrolWalkSpeed`) (`self.CharacterMovement`))
      (set `self.IsPatroling` true)
      (`self.Patrol`)
      (set `self.IsRunningBack?` false))))

(event `self.AIPerception.OnPerceptionUpdated`
  (params (UpdatedActors :type "Array of Actor Object Reference (by ref)"))
  ;[1 1 1] 플레이어 탐지를 위한 행동
  (if (and (not (`self.WasAggroed?`)) (`self.Aggressive?`))
    (for _array_element UpdatedActors
      (bind _ascb_character (cast `/Game/PlayerCharacter/Blueprints/CB_Character` _array_element))
      (`self.OnAggroPulled` _ascb_character)
      (break))))

(fn `FollowTargetDistance`
  (if (> (`KismetMathLibrary.VSize` (- (`self.StartingLocation`) (`self.K2_GetActorLocation`))) (`self.FollowPlayerRadius`))
    (`self.OnReset`)
    (return)
    (else
      (return))))

(fn `GetNextAnimation`
  (returns (Index :type Integer))
  (return (`KismetMathLibrary.RandomInteger` 2)))

(fn `InAttackRange?`
  (returns (Out :type Boolean))
  (return (<= (`self.GetDistanceTo` (`self.TargetActor`) self) (`self.AttackRange`))))

(fn `UserConstructionScript`)