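; Player character Blueprint handling mouse look, walking, strafing and jumping from input events.
; Movement handlers switch walk speed and toggle orient-to-movement and controller-yaw rotation, with strafing using ActorRotateLerp to test whether actor yaw is within a small tolerance of control yaw.
; Jumping is blocked while strafing or already flagged as jumping.
; UpdateHeadRotation derives yaw offset values but is not called in this file.
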(event `InputAxis|MouseTurn`
  (params (AxisValue :type "Float (single-precision)"))
  ;[1 1 1] 마우스 휠 회전
  (`self.AddControllerYawInput` AxisValue))

(event `InputAxis|MouseUp`
  (params (AxisValue :type "Float (single-precision)"))
  ;[1 1 1] 마우스 휠 회전
  (`self.AddControllerPitchInput` AxisValue))

(event `InputAxis|MoveForward`
  (params (AxisValue :type "Float (single-precision)"))
  (bind _charactermovement (`self.CharacterMovement`))
  ;[1 1 1] 캐릭터 이동
  (if (not (or (== (stale `InputAxis|MoveRight` AxisValue) 1.0) (== (stale `InputAxis|MoveRight` AxisValue) -1.0)))
    (if (== AxisValue 1.0)
      (set `CharacterMovementComponent.bOrientRotationToMovement` true _charactermovement)
      (set `CharacterMovementComponent.MaxWalkSpeed` 465.0 _charactermovement)
      (else
        (set `CharacterMovementComponent.bOrientRotationToMovement` false _charactermovement)
        (set `CharacterMovementComponent.MaxWalkSpeed` 225.0 _charactermovement)))
    (`self.AddMovementInput` (`KismetMathLibrary.GetForwardVector` (`KismetMathLibrary.MakeRotator` 0.0 0.0 (.yaw (`self.GetControlRotation`)))) AxisValue)))

(event `InputAxis|MoveRight`
  (params (AxisValue :type "Float (single-precision)"))
  (bind _charactermovement (`self.CharacterMovement`))
  ;[1 1 1] 캐릭터 이동
  (if (or (== AxisValue 1.0) (== AxisValue -1.0))
    (set `self.IsRightLeftMove?` true)
    (set `CharacterMovementComponent.MaxWalkSpeed` 225.0 _charactermovement)
    (if (`self.ActorRotateLerp`)
      (set `self.bUseControllerRotationYaw` true)
      (set `CharacterMovementComponent.bOrientRotationToMovement` false _charactermovement)
      (else
        (set `CharacterMovementComponent.bOrientRotationToMovement` true _charactermovement)))
    (`self.AddMovementInput` (`KismetMathLibrary.GetRightVector` (`KismetMathLibrary.MakeRotator` 0.0 0.0 (.yaw (`self.K2_GetActorRotation`)))) AxisValue)
    (else
      (set `self.IsRightLeftMove?` false)
      (if (== (stale `InputAxis|MoveForward` AxisValue) -1.0)
        (set `self.bUseControllerRotationYaw` true)
        (else
          (set `self.bUseControllerRotationYaw` false))))))

(event `InputAction|Jump`
  (params (Key :type "Key Structure"))
  ;[1 1 1] 점프
  (:`Pressed`
    (if (`self.IsJumping?`)
      _
      (elif (not (`self.IsRightLeftMove?`))
        (`self.Jump`)
        (set `self.IsJumping?` true))))
  (:`Released`
    (set `self.IsJumping?` false)))

(fn `ActorRotateLerp`
  (returns (Out :type Boolean))
  (bind (_returnvalue_roll _returnvalue_pitch _returnvalue_yaw) (`KismetMathLibrary.BreakRotator` (`self.K2_GetActorRotation`)))
  (bind (_returnvalue_roll_2 _returnvalue_pitch_2 _returnvalue_yaw_2) (`KismetMathLibrary.BreakRotator` (`self.GetControlRotation`)))
  (bind _returnvalue (`KismetMathLibrary.ClampAngle` (- _returnvalue_yaw_2 _returnvalue_yaw) -179.899994 180.0))
  (if (> _returnvalue 5.0)
    (return false)
    (elif (< _returnvalue -5.0)
      (return false)
      (else
        (return true)))))

(fn `UpdateHeadRotation`
  (locals (LocalRotate :type "Float (double-precision)" :default 60.0) (LocalActorYawOffset :type "Float (double-precision)"))
  (bind (_returnvalue_roll _returnvalue_pitch _returnvalue_yaw) (`KismetMathLibrary.BreakRotator` (`self.GetControlRotation`)))
  (bind (_returnvalue_roll_2 _returnvalue_pitch_2 _returnvalue_yaw_2) (`KismetMathLibrary.BreakRotator` (`self.K2_GetActorRotation`)))
  (bind (_returnvalue_roll_3 _returnvalue_pitch_3 _returnvalue_yaw_3) (`KismetMathLibrary.BreakRotator` (`self.GetControlRotation`)))
  (bind _localrotate (`local.LocalRotate`))
  (bind _returnvalue (`KismetMathLibrary.ClampAngle` (- _returnvalue_yaw_3 _returnvalue_yaw_2) -180.0 180.0))
  (if (not (`CharacterMovementComponent.bOrientRotationToMovement` (`self.CharacterMovement`)))
    (if (> _returnvalue _localrotate)
      _
      (elif (< _returnvalue (* _localrotate -1.0))
        (set `local.LocalActorYawOffset` (`local.LocalRotate`))))
    (else
      (set `self.DesiredActorYaw` _returnvalue_yaw))))

(fn `UserConstructionScript`)